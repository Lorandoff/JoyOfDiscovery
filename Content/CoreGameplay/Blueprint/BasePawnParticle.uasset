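; Base particle pawn that exerts mass-based, gravity-like forces on nearby physics bodies; a leading particle gets an initial force and mass scale at BeginPlay.
; OverlapSphere maintains a map of overlapping actors to their simulating components, processed every Tick.
; With AttractioN set, the pull toward the sphere follows an inverse-square falloff.
; Otherwise it still pulls inward but grows with squared distance, adding velocity-difference-based spin.
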(event OnComponentBeginOverlap(OverlapSphere)
  (params (OverlappedComponent :type Primitive%20Component%20Object%20Reference) (OtherActor :type Actor%20Object%20Reference) (OtherComp :type Primitive%20Component%20Object%20Reference) (OtherBodyIndex :type Integer) (bFromSweep :type Boolean) (SweepResult :type Hit%20Result%20Structure%20%28by%20ref%29))
  (Variables|Default|SetOverlap true)
  (if (Physics|IsSimulatingPhysics OtherComp "None")
    (Utilities|Map|Add (Variables|Default|GetOverlapCompArray) OtherActor OtherComp)))

(event OnComponentEndOverlap(OverlapSphere)
  (params (OverlappedComponent :type Primitive%20Component%20Object%20Reference) (OtherActor :type Actor%20Object%20Reference) (OtherComp :type Primitive%20Component%20Object%20Reference) (OtherBodyIndex :type Integer))
  (bind _overlapcomparray (Variables|Default|GetOverlapCompArray))
  (Utilities|Map|Remove _overlapcomparray OtherActor)
  (if (Utilities|Map|IsEmpty _overlapcomparray)
    (Variables|Default|SetOverlap false)
    (bind _values (Utilities|Map|Values _overlapcomparray))
    (for _array_element _values
      (Development|PrintString (Utilities|GetDisplayName _array_element)))))

(event EventBeginPlay
  (if (Variables|Default|GetIsLeading)
    (Physics|AddForce (Variables|Default|GetCollisionSphere) (Variables|Default|GetCForce) "None" true)
    (Class|PrimitiveComponent|SetMassScale (Variables|Default|GetCollisionSphere) "None" (Variables|Default|Getmass))))

(event Collision|EventActorBeginOverlap
  (params (OtherActor :type Actor%20Object%20Reference)))

(event EventTick
  (params (DeltaSeconds :type Float%20%28single-precision%29))
  (bind _overlapsphere (Variables|Default|GetOverlapSphere))
  (bind _returnvalue (Physics|GetMass _overlapsphere))
  (bind _returnvalue_2 (Transformation|GetWorldLocation _overlapsphere))
  (if (Variables|Default|GetOverlap)
    (bind _keys (Utilities|Map|Keys (Variables|Default|GetOverlapCompArray)))
    (for _array_element _keys
      (bind _output_get (Variables|Default|SetOtherActor _array_element))
      (Variables|Default|SetOtherComp (.Value (Utilities|Map|Find (Variables|Default|GetOverlapCompArray) _output_get)))
      (if (Variables|Default|GetAttractioN)
        (Physics|AddForce (Variables|Default|GetOtherComp) (* (/ (* (+ (* (+ (Physics|GetMass (Variables|Default|GetOtherComp)) 1.0) _returnvalue) 1.0) _returnvalue) (Class|KismetMathLibrary|VectorDistanceSquared (Transformation|GetWorldLocation (Variables|Default|GetOtherComp)) _returnvalue_2)) (Math|Vector|Normalize (- _returnvalue_2 (Transformation|GetWorldLocation (Variables|Default|GetOtherComp))) 1.0)) "None" false)
        (else
          (Physics|AddForce (Variables|Default|GetOtherComp) (* (/ (Class|KismetMathLibrary|VectorDistanceSquared (Transformation|GetWorldLocation (Variables|Default|GetOtherComp)) _returnvalue_2) (* (+ (* (+ (Physics|GetMass (Variables|Default|GetOtherComp)) 1.0) _returnvalue) 1.0) _returnvalue)) (Math|Vector|Normalize (- _returnvalue_2 (Transformation|GetWorldLocation (Variables|Default|GetOtherComp))) 1.0)) "None" false)
          (Class|PrimitiveComponent|AddAngularImpulseinDegrees (Variables|Default|GetOtherComp) (Math|Conversions|ToVector(Float) (+ (Class|KismetMathLibrary|VectorDistanceSquared (Transformation|GetVelocity) (Transformation|GetVelocity (Variables|Default|GetOtherActor))) 1.0)) "None" false))))))

(fn ConstructionScript)

(fn PythDistanceSqrt
  (params (Vec1 :type Vector) (Vec2 :type Vector))
  (bind (_x _y _z) (Class|KismetMathLibrary|BreakVector3f Vec1))
  (bind (_x_2 _y_2 _z_2) (Class|KismetMathLibrary|BreakVector3f Vec2))
  (return (Math|Float|Sqrt (+ (Math|Float|Square (- _x _x_2)) (Math|Float|Square (- _y _y_2)) (Math|Float|Square (- _z _z_2))))))