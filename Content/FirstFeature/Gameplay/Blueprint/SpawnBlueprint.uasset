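; An actor that spawns a set of small cube static mesh actors and arranges them in a ring around itself.
; BeginPlay creates ElementsCount movable cubes at the actor's transform and stores them in ElementsArray.
; The first Tick offsets each in the world YZ plane using sine and cosine of evenly stepped integer angles times Radius, guarded by IsSpawned.
; Debug arrows and printed values show the resulting positions and distances.
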(event EventBeginPlay
  (bind _returnvalue (Transformation|GetActorTransform))
  (bind (_location _rotation _scale) (Math|Transform|BreakTransform _returnvalue))
  (for _index (range 0 (- (Variables|Default|GetElementsCount) 1))
    (bind _returnvalue_2 (Game|SpawnActorfromClass (Utilities|GetClass (Variables|Default|GetStaticMeshActor)) (Math|Transform|MakeTransform _location _rotation _scale) "Undefined" "MultiplyWithRoot" 0 0))
    (Transformation|SetMobility _returnvalue_2 "Movable")
    (Components|StaticMesh|SetStaticMesh (Variables|/Script/Engine.StaticMeshActor|GetStaticMeshComponent _returnvalue_2) "/Game/Static/Models/Shapes/Shape_Cube.Shape_Cube")
    (Transformation|SetActorScale3D _returnvalue_2 "0.200000,0.200000,0.200000")
    (Utilities|Array|SetArrayElem (Variables|Default|GetElementsArray) _index _returnvalue_2 true)))

(event Collision|EventActorBeginOverlap
  (params (OtherActor :type Actor%20Object%20Reference)))

(event EventTick
  (params (DeltaSeconds :type Float%20%28single-precision%29))
  (bind _returnvalue (Transformation|GetActorLocation))
  (bind _radius (Variables|Default|GetRadius))
  (if (not (Variables|Default|GetIsSpawned))
    (for (_array_element _array_index) (Variables|Default|GetElementsArray)
      (Development|PrintString (Utilities|String|ToString(Float) (+ (* (Math|Trig|Sin(Degrees) (Math|Conversions|ToFloat(Integer) (* _array_index (/ 360 (Variables|Default|GetElementsCount))))) _radius) (.Z (Math|Vector|BreakVector (Transformation|GetActorLocation _array_element))))) true true "(R=0.000000,G=0.660000,B=1.000000,A=1.000000)" 1e+01)
      (Transformation|SetActorLocation _array_element (Math|Vector|MakeVector (.X (Math|Vector|BreakVector (Transformation|GetActorLocation _array_element))) (+ (* _radius (Math|Trig|Cos(Degrees) (Math|Conversions|ToFloat(Integer) (* _array_index (/ 360 (Variables|Default|GetElementsCount)))))) (.Y (Math|Vector|BreakVector (Transformation|GetActorLocation _array_element)))) (+ (* (Math|Trig|Sin(Degrees) (Math|Conversions|ToFloat(Integer) (* _array_index (/ 360 (Variables|Default|GetElementsCount))))) _radius) (.Z (Math|Vector|BreakVector (Transformation|GetActorLocation _array_element))))) false false)
      (Rendering|Debug|DrawDebugArrow :LineStart _returnvalue :LineEnd (Transformation|GetActorLocation _array_element) :ArrowSize 2.0 :Duration 25.0 :Thickness 2.0)
      (Development|PrintString (Utilities|String|Append (Utilities|String|ToString(Float) (Math|Vector|Distance(Vector) _returnvalue (Transformation|GetActorLocation _array_element))) ": Distance") true true "(R=0.000000,G=0.660000,B=1.000000,A=1.000000)" 15.0))
    (Variables|Default|SetIsSpawned true)))

(fn ConstructionScript)