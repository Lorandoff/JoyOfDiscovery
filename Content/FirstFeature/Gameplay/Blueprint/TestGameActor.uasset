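; Experimental physics test actor that spins and repels simulating bodies inside its Sphere1 overlap volume, and launches its own Sphere on BeginPlay unless IsRepulsed.
; Overlap events maintain an actor-to-component map that Tick iterates.
; Components spinning no faster than Rot get a clamped, distance-based sine angular impulse on Y and an inverse-distance outward push.
; GravitationForce, NewFunction and many disconnected nodes are unused experiments.
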(event OnComponentBeginOverlap(Sphere1)
  (params (OverlappedComponent :type Primitive%20Component%20Object%20Reference) (OtherActor :type Actor%20Object%20Reference) (OtherComp :type Primitive%20Component%20Object%20Reference) (OtherBodyIndex :type Integer) (bFromSweep :type Boolean) (SweepResult :type Hit%20Result%20Structure%20%28by%20ref%29))
  (if (and (Physics|IsSimulatingPhysics OtherComp "None") (not (== (Variables|Default|GetSphere) OtherComp)))
    (Utilities|Map|Add (Variables|Default|GetOverlapCompArray) OtherActor OtherComp)
    (Variables|Default|SetIsOverlapped true)))

(event OnComponentEndOverlap(Sphere1)
  (params (OverlappedComponent :type Primitive%20Component%20Object%20Reference) (OtherActor :type Actor%20Object%20Reference) (OtherComp :type Primitive%20Component%20Object%20Reference) (OtherBodyIndex :type Integer))
  (bind _overlapcomparray (Variables|Default|GetOverlapCompArray))
  (Utilities|Map|Remove _overlapcomparray OtherActor)
  (if (Utilities|Map|IsEmpty _overlapcomparray)
    (Variables|Default|SetIsOverlapped false)))

(event EventBeginPlay
  (bind _cforce (Variables|Default|GetCForce))
  (if (not (Variables|Default|GetIsRepulsed))
    (Physics|AddForce (Variables|Default|GetSphere) _cforce "None" true)
    (Physics|AddImpulse (Variables|Default|GetSphere) _cforce "None" true)))

(event Collision|EventActorBeginOverlap
  (params (OtherActor :type Actor%20Object%20Reference)))

(event EventTick
  (params (DeltaSeconds :type Float%20%28single-precision%29))
  (bind _sphere (Variables|Default|GetSphere))
  (bind _rot (Variables|Default|GetRot))
  (if (Variables|Default|GetIsOverlapped)
    (bind _keys (Utilities|Map|Keys (Variables|Default|GetOverlapCompArray)))
    (for _array_element _keys
      (bind _output_get (Variables|Default|SetOtherActor _array_element))
      (bind _output_get_2 (Variables|Default|SetOtherComp (.Value (Utilities|Map|Find (Variables|Default|GetOverlapCompArray) _output_get))))
      (if (<= (Math|Vector|VectorLength (Physics|GetPhysicsAngularVelocityinDegrees _output_get_2 "None")) _rot)
        (bind _resultforce (CallFunction|Rotation (Variables|Default|GetImpulseRot) _rot _output_get_2))
        (bind _resultforce_2 (CallFunction|SineForce _resultforce true _output_get_2 _sphere 3.0))
        (Class|PrimitiveComponent|AddAngularImpulseinDegrees _output_get_2 _resultforce_2 "None" true)
        (bind _force (CallFunction|OneOverForce "0, 0, 0" _sphere _output_get_2))
        (Physics|AddForce _output_get_2 _force "None" true)))))

(fn ConstructionScript)

(fn NewFunction)

(fn Rotation
  (params (ImpulseRotValue :type Vector) (RotThreshold :type Float%20%28double-precision%29) (Object :type Primitive%20Component%20Object%20Reference))
  (bind (_x _y _z) (Math|Vector|BreakVector ImpulseRotValue))
  (if true
    (return (Math|Vector|MakeVector (Math|Float|Clamp(Float) _x -1.0) (Math|Float|Clamp(Float) _y -1.0) (Math|Float|Clamp(Float) _z -1.0)))))

(fn GravitationForce
  (params (OtherComp :type Primitive%20Component%20Object%20Reference) (OwnComp :type Primitive%20Component%20Object%20Reference) (IsActractive :type Boolean))
  (bind _returnvalue (Physics|GetMass OwnComp))
  (bind _returnvalue_2 (Physics|GetMass OtherComp))
  (bind _returnvalue_3 (Transformation|GetWorldLocation OwnComp))
  (bind _returnvalue_4 (Transformation|GetWorldLocation OtherComp))
  (bind _returnvalue_5 (Math|Vector|Distance(Vector) _returnvalue_3 _returnvalue_4))
  (bind _returnvalue_6 (* _returnvalue_2 _returnvalue))
  (bind _returnvalue_7 (- _returnvalue_4 _returnvalue_3))
  (bind _returnvalue_8 (Math|Vector|Normalize _returnvalue_7 1.0))
  (bind _returnvalue_9 (/ _returnvalue_6 _returnvalue_5))
  (bind _returnvalue_10 (* _returnvalue_9 _returnvalue_8))
  (if IsActractive
    (return _returnvalue_10)
    (else
      (return (Math|Vector|NegateVector _returnvalue_10)))))

(fn SineForce
  (params (ForceValue :type Vector) (IsExpansion :type Boolean) (OtherComp :type Primitive%20Component%20Object%20Reference) (OwnComp :type Primitive%20Component%20Object%20Reference) (Period :type Float%20%28double-precision%29))
  (bind _returnvalue (Transformation|GetWorldLocation OwnComp))
  (bind _returnvalue_2 (Transformation|GetWorldLocation OtherComp))
  (bind _returnvalue_3 (Math|Vector|Distance(Vector) _returnvalue_2 _returnvalue))
  (bind _returnvalue_4 (/ _returnvalue_3 Period))
  (bind _returnvalue_5 (Math|Trig|Sin(Degrees) _returnvalue_4))
  (bind _returnvalue_6 (Math|Vector|MakeVector 0.0 _returnvalue_5 0.0))
  (bind _returnvalue_7 (* _returnvalue_6 ForceValue))
  (bind (_x _y _z) (Math|Vector|BreakVector _returnvalue_7))
  (if IsExpansion
    (return (Math|Vector|MakeVector (Math|Float|Clamp(Float) _x -1.0) (Math|Float|Clamp(Float) _y -1.0) (Math|Float|Clamp(Float) _z -1.0)))
    (else
      (return _returnvalue_6))))

(fn OneOverForce
  (params (Force%20Value :type Vector) (OwnComp :type Primitive%20Component%20Object%20Reference) (OtherComp :type Primitive%20Component%20Object%20Reference))
  (bind _returnvalue (Transformation|GetWorldLocation OtherComp))
  (bind _returnvalue_2 (Transformation|GetWorldLocation OwnComp))
  (return (* (Math|Vector|Normalize (- _returnvalue _returnvalue_2) 1.0) (/ 1.0 (Math|Vector|Distance(Vector) _returnvalue _returnvalue_2)))))